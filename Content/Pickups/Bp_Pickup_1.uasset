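; Pickup actor that grants the third-person character a random ability when the character overlaps it.
; On overlap it casts to BP_ThirdPersonCharacter, then picks one of five outcomes at random.
; Only the first two set character flags, enabling grapple or overclock; the other three just print debug messages.
; Every outcome ends by destroying the pickup.
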(event `self.ReceiveActorBeginOverlap`
  (params (OtherActor :type "Actor Object Reference"))
  (bind _asbp_third_person_character (cast `/Game/ThirdPerson/Blueprints/BP_ThirdPersonCharacter` OtherActor))
  (`KismetSystemLibrary.PrintString` "pickup....picked up?")
  (switch `int` (`KismetMathLibrary.RandomInteger` 5)
    (:`0`
      (`KismetSystemLibrary.PrintString` "hey you got the first ability (grapple)")
      (set `/Game/ThirdPerson/Blueprints/BP_ThirdPersonCharacter.Grapple_YN` true _asbp_third_person_character))
    (:`1`
      (`KismetSystemLibrary.PrintString` "hey you got the second ability (overclock)")
      (set `/Game/ThirdPerson/Blueprints/BP_ThirdPersonCharacter.OverClock_YN` true _asbp_third_person_character))
    (:`2`
      (`KismetSystemLibrary.PrintString` "hey you got the third ability"))
    (:`3`
      (`KismetSystemLibrary.PrintString` "hey you got the fourth ability"))
    (:`4`
      (`KismetSystemLibrary.PrintString` "hey you got the fith ability")))
  (`self.K2_DestroyActor`))

(fn `UserConstructionScript`)